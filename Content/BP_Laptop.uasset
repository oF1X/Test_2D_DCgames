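; Laptop actor that accepts an opened USB stick, making it appear plugged in at a fixed spot.
; When its Box overlaps a component named "shteker" on a BP_USB whose IsOpened flag is set, it spawns a replacement USB at a hardcoded world transform.
; The replacement copies the original's body material and is marked opened, then the original is destroyed.
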(event OnComponentBeginOverlap(Box)
  (params (OverlappedComponent :type Primitive%20Component%20Object%20Reference) (OtherActor :type Actor%20Object%20Reference) (OtherComp :type Primitive%20Component%20Object%20Reference) (OtherBodyIndex :type Integer) (bFromSweep :type Boolean) (SweepResult :type Hit%20Result%20Structure%20%28by%20ref%29))
  (if (Utilities|Enum|Equal(Enum) (Utilities|String|ToString(Object) OtherComp) "shteker")
    (Utilities|IsValid OtherActor
      (:Is%20Valid
        (bind _asbp_usb (Utilities|Casting|CastToBP_USB OtherActor))
        (if (Variables|/Game/BP_USB.BP_USB_C|GetIsOpened _asbp_usb)
          (bind _returnvalue (Game|SpawnActorfromClass "/Game/BP_USB.BP_USB_C" (Math|Transform|MakeTransform "1724.399046,1607.060572,87.153160" "0.000000,40.000000,0.000000" "0.750000,0.750000,0.750000") "Undefined" "MultiplyWithRoot" 0 0))
          (Rendering|Material|SetMaterial (Variables|/Game/BP_USB.BP_USB_C|GetSM_USBBody _returnvalue) 0 (Rendering|Material|GetMaterial (Variables|/Game/BP_USB.BP_USB_C|GetSM_USBBody _asbp_usb) 0))
          (Variables|/Game/BP_USB.BP_USB_C|SetIsOpened _returnvalue true)
          (Actor|DestroyActor _asbp_usb))))))

(event EventBeginPlay)

(event Collision|EventActorBeginOverlap
  (params (OtherActor :type Actor%20Object%20Reference)))

(event EventTick
  (params (DeltaSeconds :type Float%20%28single-precision%29)))

(fn ConstructionScript)