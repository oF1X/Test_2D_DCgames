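; BP_FaunderMain is an actor that spawns a color-matched BP_USB on demand.
; Its construction script gives the Cylinder a random yellow, purple or blue material.
; SpawnUsb destroys every existing BP_USB, spawns a replacement at a hardcoded world transform and copies the Cylinder's material onto the new USB body.
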(event Custom|SpawnUsb
  (bind _outactors (Actor|GetAllActorsOfClass "/Game/BP_USB.BP_USB_C"))
  (for _array_element _outactors
    (Utilities|IsValid _array_element
      (:Is%20Valid
        (Actor|DestroyActor _array_element))))
  (bind _returnvalue (Game|SpawnActorfromClass "/Game/BP_USB.BP_USB_C" (Math|Transform|MakeTransform "1856.707108,1641.886255,87.334558" "0.000000,40.000000,0.000000" "0.750000,0.750000,0.750000") "Undefined" "MultiplyWithRoot" 0 0))
  (Rendering|Material|SetMaterial (Variables|/Game/BP_USB.BP_USB_C|GetSM_USBBody _returnvalue) 0 (Rendering|Material|GetMaterial (Variables|Default|GetCylinder) 0)))

(fn ConstructionScript
  (Rendering|Material|SetMaterial (Variables|Default|GetCylinder) 0 (.OutItem (Utilities|Array|Random (Utilities|Array|MakeArray "/Game/M_Yellow.M_Yellow" "/Game/M_Purple.M_Purple" "/Game/M_Blue.M_Blue")))))