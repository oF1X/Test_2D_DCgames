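; BP_USB is a USB stick actor with a detachable cap and an opened state.
; Event_DetachCap reattaches the cap to the root keeping world transform, enables its physics with SixDOF constraint mode, sets IsOpened and turns Colored green.
; The construction script shows instances already opened as green with the cap hidden.
; Clicks on the body toggle IsDragging, but the cursor-follow and spin logic is disconnected, leaving Tick empty.
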(event OnClicked(SM_USBBody)
  (params (TouchedComponent :type Primitive%20Component%20Object%20Reference) (ButtonPressed :type Key%20Structure :default "None"))
  (Variables|Default|SetIsDragging true))

(event OnReleased(SM_USBBody)
  (params (TouchedComponent :type Primitive%20Component%20Object%20Reference) (ButtonReleased :type Key%20Structure :default "None"))
  (Variables|Default|SetIsDragging false))

(event Custom|OnClicked_Event
  (params (TouchedActor :type Actor%20Object%20Reference) (ButtonPressed :type Key%20Structure :default "None"))
  (Variables|Default|SetIsDragging true))

(event Custom|Event_DetachCap
  (bind _sm_cap (Variables|Default|GetSM_Cap))
  (Transformation|AttachComponentToComponent _sm_cap (Variables|Default|GetDefaultSceneRoot) "None" "KeepWorld" "KeepWorld" "KeepWorld" true)
  (Physics|SetSimulatePhysics _sm_cap true)
  (Variables|Default|SetIsOpened true)
  (Rendering|Material|SetMaterial (Variables|Default|Getcolored) 0 "/Game/M_Green.M_Green")
  (Class|PrimitiveComponent|SetConstraintMode _sm_cap "SixDOF"))

(event EventTick
  (params (DeltaSeconds :type Float%20%28single-precision%29)))

(fn ConstructionScript
  (if (Variables|Default|GetIsOpened)
    (Rendering|Material|SetMaterial (Variables|Default|Getcolored) 0 "/Game/M_Green.M_Green")
    (Rendering|SetVisibility (Variables|Default|GetSM_Cap) false false)))